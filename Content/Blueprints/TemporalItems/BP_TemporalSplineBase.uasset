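; Base Blueprint for temporal items: moves a static mesh along a spline over a configurable completion time, starting at BeginPlay.
; A timeline drives position by spline distance, optionally matching spline rotation.
; AutoReverse ping-pongs endlessly via a FlipFlop; otherwise the mesh travels once, and Interact rewinds it to the start, from where it replays forward.
; Getters expose separate flags for general and user interactability.
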(event `self.ReceiveBeginPlay`
  (`self.MoveAlongSpline`))

(event `MoveAlongSpline`
  (`TimelineComponent.SetPlayRate` (`self.Timeline`) (/ 1.0 (`self.TimeToComplete`)))
  (if (`self.autoReverse`)
    (`/Engine/EditorBlueprintResources/StandardMacros.FlipFlop`
      (:`A`
        (bind (_direction _newtrack_0) (`Timeline|Timeline` :!label _label)
          (:`Update`
            (if (`self.followSplineRotation`)
              (bind _returnvalue (`KismetMathLibrary.Lerp` 0.0 (`SplineComponent.GetSplineLength` (`self.Spline`)) _newtrack_0))
              (bind _returnvalue_2 (`SplineComponent.GetLocationAtDistanceAlongSpline` (`self.Spline`) _returnvalue "World"))
              (`SceneComponent.K2_SetWorldTransform` (`self.StaticMesh`) (`KismetMathLibrary.MakeTransform` _returnvalue_2 (`SplineComponent.GetRotationAtDistanceAlongSpline` (`self.Spline`) _returnvalue "World")) false false)
              (else
                (`SceneComponent.K2_SetWorldLocation` (`self.StaticMesh`) _returnvalue_2 false false))))
          (:`Finished`
            (if (`self.temporalRecall`)
              (`self.MoveAlongSpline`)
              (set `self.temporalRecall` false)
              (elif (`self.autoReverse`)
                (`self.MoveAlongSpline`))))))
      (:`B`
        (goto _label :!via `Reverse`)))
    (else
      (goto _label))))

(event `/Game/GameData/Interface/BI_TemporalInteract.Interact`
  (if (not (`self.autoReverse`))
    (set `self.temporalRecall` true)
    (goto _label :!via `Reverse`)))

(fn `getCanInteract`
  (returns (`canInteract?` :type Boolean))
  (return (`self.Can Interact?`)))

(fn `getCanUserInteract`
  (returns (`UserInteract?` :type Boolean))
  (return (`self.User Interact?`)))

(fn `UserConstructionScript`)