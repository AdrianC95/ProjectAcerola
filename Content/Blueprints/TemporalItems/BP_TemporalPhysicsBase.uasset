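; Base Blueprint for a physics object that records its movement and rewinds along that path when interacted with.
; A looping timer stores the mesh transform every 0.1 seconds until the tracking limit, then freezes physics, optionally auto-reverting.
; Rewind disables simulation and replays the Reverse timeline per stored transform, lerping backwards at a RevertTime-based rate.
; When done, it clears history, resumes tracking and re-enables physics after a short delay.
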(event `/Game/GameData/Interface/BI_TemporalInteract.Interact`
  (bind _tracktimer (`self.TrackTimer`))
  (bind _staticmesh (`self.StaticMesh`))
  (`TimelineComponent.SetPlayRate` (`self.Reverse`) (/ 1.0 (`self.RevertTime`)) :!label _label)
  (if (`KismetSystemLibrary.K2_IsTimerActiveHandle` _tracktimer)
    (`KismetSystemLibrary.K2_PauseTimerHandle` _tracktimer)
    (`PrimitiveComponent.SetSimulatePhysics` (`self.StaticMesh`) false))
  (set `self.Previous` (`SceneComponent.K2_GetComponentToWorld` (`self.StaticMesh`)) :!label _label_2)
  (bind (_direction _revert) (`Timeline|Reverse` :!via `PlayFromStart`)
    (:`Update`
      (`SceneComponent.K2_SetWorldTransform` (`self.StaticMesh`) (`KismetMathLibrary.TLerp` (`self.Previous`) (`|GetArrayItem` (`self.PreviousTransform`) (`self.TotalItems`)) _revert) false false))
    (:`Finished`
      (bind _result (`/Engine/EditorBlueprintResources/StandardMacros.DecrementInt` (`self.TotalItems`))
        (:`  `
          (if (== _result 0)
            (`|ExecutionSequence`
              (:`then_0`
                (`PrimitiveComponent.SetPhysicsLinearVelocity` _staticmesh (0.0 0.0 0.0) false "None")
                (`KismetSystemLibrary.Delay` 0.5)
                (`PrimitiveComponent.SetSimulatePhysics` _staticmesh true))
              (:`then_1`
                (`KismetSystemLibrary.K2_UnPauseTimerHandle` (`self.TrackTimer`)))
              (:`then_2`
                (`KismetArrayLibrary.Array_Clear` (`self.PreviousTransform`))))
            (else
              (goto _label_2))))))))

(event `AutoRevert`
  (goto _label))

(event `self.ReceiveBeginPlay`
  (bind _returnvalue (`KismetSystemLibrary.K2_SetTimer` null "TrackTransform" 0.1 true))
  (set `self.TrackTimer` _returnvalue)
  (set `self.MaxTrackingIndex` (- (/ (`self.SecondsToTrack`) 0.1) 1)))

(event `TrackTransform`
  (bind _returnvalue (`KismetArrayLibrary.Array_Add` (`self.PreviousTransform`) (`SceneComponent.K2_GetComponentToWorld` (`self.StaticMesh`))))
  (set `self.TotalItems` _returnvalue)
  (if (== _returnvalue (`self.MaxTrackingIndex`))
    (`PrimitiveComponent.SetSimulatePhysics` (`self.StaticMesh`) false)
    (`KismetSystemLibrary.K2_PauseTimerHandle` (`self.TrackTimer`))
    (if (`self.autoRevert?`)
      (`self.AutoRevert`))))

(fn `getCanInteract`
  (returns (`canInteract?` :type Boolean))
  (return (`self.Can Interact?`)))

(fn `getCanUserInteract`
  (returns (`UserInteract?` :type Boolean))
  (return (`self.User Interact?`)))

(fn `UserConstructionScript`)