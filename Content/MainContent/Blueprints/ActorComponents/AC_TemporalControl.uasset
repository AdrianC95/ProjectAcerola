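; Actor component that records a mesh's world transforms and rewinds the mesh back along them.
; ActorTracker appends each transform to an array and advances an index, storing the caller's timer handle.
; TR_StartCall pauses tracking and steps the index back, while TemporalRetrace lerps toward that entry using a supplied alpha.
; TR_FinishUpdate pauses reversal and resumes tracking at index 1, without trimming the array.
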(event `ActorTracker`
  (params (Mesh :type "StaticMeshComponent Object Reference") (Timer :type "TimerHandle Structure"))
  (set `self.MeshRef` Mesh)
  (if (`KismetSystemLibrary.K2_IsValidTimerHandle` Timer)
    (set `self.TrackingTimer` Timer))
  (`KismetArrayLibrary.Array_Add` (`self.TransformTrack`) (`SceneComponent.K2_GetComponentToWorld` (`self.MeshRef`)))
  (`/Engine/EditorBlueprintResources/StandardMacros.IncrementInt` (`self.ArrayIndex`)))

(event `TemporalRetrace`
  (params (Alpha :type "Float (single-precision)"))
  (`SceneComponent.K2_SetWorldTransform` (`self.MeshRef`) (`KismetMathLibrary.TLerp` (`self.PreviousTransform`) (`|GetArrayItem` (`self.TransformTrack`) (`self.ArrayIndex`)) Alpha) false false))

(event `TR_StartCall`
  (params (Timer :type "TimerHandle Structure"))
  (bind _trackingtimer (`self.TrackingTimer`))
  (set `self.PreviousTransform` (`SceneComponent.K2_GetComponentToWorld` (`self.MeshRef`)))
  (`/Engine/EditorBlueprintResources/StandardMacros.DecrementInt` (`self.ArrayIndex`)
    (:`  `
      (if (`KismetSystemLibrary.K2_IsValidTimerHandle` Timer)
        (set `self.ReverseTimer` Timer))
      (if (`KismetSystemLibrary.K2_IsTimerActiveHandle` _trackingtimer)
        (`KismetSystemLibrary.K2_PauseTimerHandle` _trackingtimer)))))

(event `TR_FinishUpdate`
  (if (== (`self.ArrayIndex`) 1)
    (`KismetSystemLibrary.K2_PauseTimerHandle` (`self.ReverseTimer`))
    (`KismetSystemLibrary.K2_UnPauseTimerHandle` (`self.TrackingTimer`))
    (`KismetSystemLibrary.PrintString` "Hello")))